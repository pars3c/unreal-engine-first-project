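; Player actor Blueprint that initializes health and plays a spawn animation at BeginPlay.
; It sets Health to MaxHealth and stores the mesh's starting pitch and the actor's spawn location.
; The SpawnAnimation timeline then slides the actor from that location along +Y without sweeping, while setting PlayerMesh's relative rotation from a rotator lerp.
; Tick and the construction script are empty.
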(event EventBeginPlay
  (Variables|Floats|SetHealth (Variables|Floats|GetMaxHealth))
  (Variables|Floats|SetPitch (.Pitch (Math|Rotator|BreakRotator (Variables|/Script/Engine.SceneComponent|GetRelativeRotation (Variables|Default|GetPlayerMesh)))))
  (Variables|Vectors|SetSpawnLocation (Transformation|GetActorLocation))
  (bind _spawn (Timeline|SpawnAnimation Play)
    (:Update
      (Transformation|SetActorLocation (Math|Vector|Lerp(Vector) (Variables|Vectors|GetSpawnLocation) (+ (Variables|Vectors|GetSpawnLocation) "0,1000.000000, 0") _spawn) false false)
      (Transformation|SetRelativeRotation (Variables|Default|GetPlayerMesh) (Math|Rotator|Lerp(Rotator) "0, 0, 0" "0, 0, 0" 0.0) false false))))

(event EventTick
  (params (DeltaSeconds :type Float%20%28single-precision%29)))

(fn ConstructionScript)